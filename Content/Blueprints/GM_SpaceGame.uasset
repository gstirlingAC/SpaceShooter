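; GM_SpaceGame is the space game's game mode, handling the main menu and player ship spawning.
; On BeginPlay it creates the main menu widget, stores a reference and shows it with a mouse cursor and UI-only input.
; Separate events hide the menu, restoring game-only input, and spawn BP_PlayerShip; neither is called within this Blueprint.
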(event `Spawn Player`
  (`|SpawnActorFromClass` "/Game/Blueprints/BP_PlayerShip.BP_PlayerShip_C" (`KismetMathLibrary.MakeTransform` (0.0 0.0 0.0)) "Undefined" "MultiplyWithRoot" null null))

(event `Hide Main Menu`
  (bind _returnvalue (`GameplayStatics.GetPlayerController` 0))
  ;[1 1 1] Hide main menu and remove it from the viewport
  (set `PlayerController.bShowMouseCursor` false _returnvalue)
  (`WidgetBlueprintLibrary.SetInputMode_GameOnly` _returnvalue)
  (`Widget.RemoveFromParent` (`self.W Main Menu Ref`)))

(event `Show Main Menu`
  (bind _returnvalue (`GameplayStatics.GetPlayerController` 0))
  (bind _w_main_menu_ref (`self.W Main Menu Ref`))
  ;[1 1 1] Display main menu and disable input on everything except UI
  (set `PlayerController.bShowMouseCursor` true _returnvalue)
  (`WidgetBlueprintLibrary.SetInputMode_UIOnlyEx` _returnvalue _w_main_menu_ref)
  (`UserWidget.AddToViewport` _w_main_menu_ref 0))

(event `self.ReceiveBeginPlay`
  ;[1 1 1] Create widget and show it
  (bind _returnvalue (`|CreateWidget` "/Game/UI/W_MainMenu.W_MainMenu_C" (`GameplayStatics.GetPlayerController` 0)))
  (set `self.W Main Menu Ref` _returnvalue)
  (`self.Show Main Menu`))

(fn `UserConstructionScript`)